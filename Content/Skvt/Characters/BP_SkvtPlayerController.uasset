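; Player controller for the Skvt game that handles pawn swapping and a pausing main menu.
; On BeginPlay it adds Enhanced Input mapping contexts for default, crouch, swap and menu input.
; The swap action possesses the next pawn from all pawns in the level, wrapping to the first.
; The menu action toggles WBP_MainMenu, switching input mode, pause state and mouse cursor.
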(event `self.ReceiveBeginPlay`
  (bind _returnvalue (pcsubsystem `EnhancedInputLocalPlayerSubsystem` self))
  (`/Engine/EditorBlueprintResources/StandardMacros.IsValid` _returnvalue
    (:`Is Valid`
      (`EnhancedInputSubsystemInterface.AddMappingContext` _returnvalue "/Game/ThirdPerson/Input/IMC_Default.IMC_Default" 0 (struct))
      (`EnhancedInputSubsystemInterface.AddMappingContext` _returnvalue "/Game/Skvt/Characters/Input/IMC_Crouch.IMC_Crouch" 0 (struct))
      (`EnhancedInputSubsystemInterface.AddMappingContext` _returnvalue "/Game/Skvt/Characters/Input/IMC_SwapPawn.IMC_SwapPawn" 0 (struct))
      (`EnhancedInputSubsystemInterface.AddMappingContext` _returnvalue "/Game/Skvt/Characters/Input/IMC_MainMenu.IMC_MainMenu" 0 (struct)))))

(event `EnhancedInput|/Game/Skvt/Characters/Input/Actions/IA_Swap`
  (params (ActionValue :type Boolean) (ElapsedSeconds :type "Float (double-precision)") (TriggeredSeconds :type "Float (double-precision)") (InputAction :type "InputAction Object Reference" :default "/Game/Skvt/Characters/Input/Actions/IA_Swap.IA_Swap"))
  (:`Triggered`
    (bind _outactors (`GameplayStatics.GetAllActorsOfClass` "/Script/Engine.Pawn"))
    (bind _selected_pawn (`self.GetPawnToPosses` _outactors))
    (`self.Possess` _selected_pawn)))

(event `EnhancedInput|/Game/Skvt/Characters/Input/Actions/IA_Open_Menu`
  (params (ActionValue :type Boolean) (ElapsedSeconds :type "Float (double-precision)") (TriggeredSeconds :type "Float (double-precision)") (InputAction :type "InputAction Object Reference" :default "/Game/Skvt/Characters/Input/Actions/IA_Open_Menu.IA_Open_Menu"))
  (:`Triggered`
    (if (`self.IsMainMenuOpen`)
      (`self.CloseMainMenu`)
      (else
        (`self.Create Main Menu`)))))

(fn `CloseMainMenu`
  (`Widget.RemoveFromParent` (`self.MenuWidget`))
  (set `self.MenuWidget` null)
  (`WidgetBlueprintLibrary.SetInputMode_GameOnly` self)
  (`GameplayStatics.SetGamePaused` false)
  (set `self.bShowMouseCursor` false))

(fn `Create Main Menu`
  (bind _returnvalue (`|CreateWidget` "/Game/Skvt/UI/Widgets/Menu/WBP_MainMenu.WBP_MainMenu_C" self))
  (bind _output_get (set `self.MenuWidget` _returnvalue))
  (`UserWidget.AddToViewport` _output_get 0)
  (`WidgetBlueprintLibrary.SetInputMode_GameAndUIEx` self _output_get)
  (`GameplayStatics.SetGamePaused` true)
  (set `self.bShowMouseCursor` true))

(fn `GetPawnToPosses`
  (params (PawnArray :type "Array of Pawn Object Reference"))
  (returns (`Selected Pawn` :type "Pawn Object Reference"))
  (bind _returnvalue (+ (`KismetArrayLibrary.Array_Find` PawnArray (`self.K2_GetPawn`)) 1))
  (if (`KismetArrayLibrary.Array_IsValidIndex` PawnArray _returnvalue)
    (return (`|GetArrayItem` PawnArray _returnvalue))
    (else
      (return (`|GetArrayItem` PawnArray)))))

(fn `IsMainMenuOpen`
  (returns (IsOpen :type Boolean))
  (return (`KismetSystemLibrary.IsValid` (`self.MenuWidget`))))

(fn `UserConstructionScript`)