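; BP_WallSconce is a wall sconce light actor that can be switched on and off.
; The construction script applies exposed brightness, color and inner and outer cone angles to the SconceLight component, then sets its initial state from IsLit.
; TurnOn and TurnOff events call UpdateLight, which stores IsLit and toggles the light component's visibility.
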(event `/Game/Skvt/Blueprints/BPI_ElectronicDevice.TurnOff`
  (`self.Update Light` false))

(event `/Game/Skvt/Blueprints/BPI_ElectronicDevice.TurnOn`
  (`self.Update Light` true))

(fn `Initialize Light`
  (bind _sconcelight (`self.SconceLight`))
  (`LightComponent.SetIntensity` _sconcelight (`self.Brightness`))
  (`LightComponent.SetLightColor` _sconcelight (`self.Color`) true)
  (`SpotLightComponent.SetInnerConeAngle` _sconcelight (`self.Inner Cone Angle`))
  (`SpotLightComponent.SetOuterConeAngle` _sconcelight (`self.Outer Cone Angle`)))

(fn `Update Light`
  (params (isOn :type Boolean))
  (bind _output_get (set `self.isLit` isOn))
  (`SceneComponent.SetVisibility` (`self.SconceLight`) _output_get false))

(fn `UserConstructionScript`
  (`self.Initialize Light`)
  (`self.Update Light` (`self.isLit`)))